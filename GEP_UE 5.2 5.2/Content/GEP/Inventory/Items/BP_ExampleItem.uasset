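; BP_ExampleItem is an example inventory item that can be picked up into the player's inventory.
; Its Pickup event finds BP_PlayerCharacter with GetActorOfClass and passes the row name and quantity from BPItemData to BPInventorySystem's AddToInventory.
; The item destroys itself when the add succeeds and prints debug messages for success or an invalid inventory.
; A disconnected data table lookup that prints the item name never runs.
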(event EventPickup
  (bind _bp_itemdata (Variables|Default|GetBP_ItemData))
  (bind _returnvalue (Actor|GetActorOfClass "/Game/GEP/Blueprints/Essentials/BP_PlayerCharacter.BP_PlayerCharacter_C"))
  (Utilities|IsValid (Variables|/Game/GEP/Blueprints/Essentials/BP_PlayerCharacter.BP_PlayerCharacter_C|GetBP_InventorySystem _returnvalue)
    (:Is%20Valid
      (bind _success (Default|AddtoInventory (Variables|/Game/GEP/Blueprints/Essentials/BP_PlayerCharacter.BP_PlayerCharacter_C|GetBP_InventorySystem _returnvalue) (.rowname (Variables|/Game/GEP/Inventory/BP_ItemData.BP_ItemData_C|GetItemID _bp_itemdata)) (Variables|/Game/GEP/Inventory/BP_ItemData.BP_ItemData_C|GetItemQuantity _bp_itemdata)))
      (if _success
        (Development|PrintString "Working!")
        (Actor|DestroyActor)))
    (:Is%20Not%20Valid
      (Development|PrintString "Something is invalid"))))

(fn ConstructionScript)